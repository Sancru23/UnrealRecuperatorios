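; Actor component that tracks its owner's health and handles death, starting at max health on BeginPlay.
; GetDamage ignores its NewDamage input, subtracts a fixed clamped amount and plays a damage sound.
; At zero health it replaces all widgets with the lose menu, shows the cursor, sets game-only input and destroys the owner.
; A dynamic material gradient branch in GetDamage is disconnected and never runs.
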(event EventBeginPlay
  (Variables|Default|SetHealt (Variables|Default|GetMaxHealth)))

(fn GetDamage
  (params (NewDamage :type Float%20%28double-precision%29))
  (bind _returnvalue (Game|GetPlayerController 0))
  (bind _output_get (Variables|Default|SetHealt (Math|Float|Clamp(Float) (- (Variables|Default|GetHealt) 2e+01) 0.0 (Variables|Default|GetMaxHealth))))
  (Audio|PlaySound2D "/Game/StarterContent/Audio/TakeDamage.TakeDamage" 1.0 1.0 0.0 0 0)
  (if (== _output_get 0.0)
    (Viewport|RemoveAllWidgets)
    (bind _returnvalue_2 (UserInterface|CreateWidget "/Game/ThirdPerson/Blueprints/LoseMenu.LoseMenu_C"))
    (UserInterface|Viewport|AddtoViewport _returnvalue_2 0)
    (Variables|/Script/Engine.PlayerController|SetbShowMouseCursor _returnvalue true)
    (Input|SetInputModeGameOnly _returnvalue false)
    (Actor|DestroyActor (Components|GetOwner))))