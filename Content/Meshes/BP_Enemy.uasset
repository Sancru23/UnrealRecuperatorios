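; Enemy character base that configures damage, attack range, scale, life, mesh and debug color from a data table row keyed by its Type enum.
; AI perception writes SuccessfullySensed directly into the CantSeePlayer blackboard key, despite its inverted name.
; A looping timer draws a debug box for attack range at a billboard, which construction offsets by AttackRange before the row loads.
; The walk speed assignment is disconnected.
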(event OnTargetPerceptionUpdated(AIPerception)
  (params (Actor :type Actor%20Object%20Reference) (Stimulus :type AI%20Stimulus%20Structure))
  (AI|Components|Blackboard|SetValueasBool (AI|GetBlackboard 0) (Utilities|Name|MakeLiteralName "CantSeePlayer") (.bSuccessfullySensed (Utilities|Struct|BreakAIStimulus Stimulus))))

(event Custom|linear
  (bind _capsulecomponent (Variables|Collision|GetCapsuleComponent))
  (Rendering|Debug|DrawDebugBox (Transformation|GetWorldLocation (Variables|Default|GetBillboard)) (Math|Vector|MakeVector (Variables|Default|GetAttackRange) (* (Components|Capsule|GetScaledCapsuleRadius _capsulecomponent) 2.0) (* (Components|Capsule|GetScaledCapsuleHalfHeight _capsulecomponent) 2.0)) (Variables|Default|Getcolor) (Transformation|GetActorRotation) 2.0 2.0))

(event EventBeginPlay
  (CallFunction|LoadValue)
  (Utilities|Time|SetTimerbyEvent (delegate Custom|linear) 2.0 true))

(fn ConstructionScript
  (Transformation|SetRelativeLocation (Variables|Default|GetBillboard) (Math|Vector|MakeVector (Variables|Default|GetAttackRange) 0.0 0.0) false false))

(fn LoadValue
  (bind _returnvalue (Utilities|GetDataTableRow "/Game/Blueprints/NewDataTable.NewDataTable" (Utilities|String|StringToName (Utilities|String|EnumtoString (Variables|Default|GetType))))
    (:then
      (Variables|Default|SetDamage (.Damage (Utilities|Struct|BreakF_EnemyData _returnvalue)))
      (Variables|Default|SetAttackRange (.attackRange (Utilities|Struct|BreakF_EnemyData _returnvalue)))
      (Transformation|SetActorScale3D (Math|Conversions|ToVector(Float) (.Scale (Utilities|Struct|BreakF_EnemyData _returnvalue))))
      (Variables|Default|SetCurrentLife (.CurrentLife (Utilities|Struct|BreakF_EnemyData _returnvalue)))
      (Components|SkeletalMesh|SetSkeletalMeshAsset (Variables|Character|GetMesh) (.Mesh (Utilities|Struct|BreakF_EnemyData _returnvalue)))
      (Variables|Default|Setcolor (.DebugColor (Utilities|Struct|BreakF_EnemyData _returnvalue))))))