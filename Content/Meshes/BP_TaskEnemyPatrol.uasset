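; Behavior tree task that gives an AI-controlled enemy its next patrol destination.
; On execute, it picks a random reachable navmesh point within a fixed radius of the owning controller's location, writes it to the BBloc blackboard key and finishes successfully.
; An unconnected branch holds an alternative waypoint patrol that steps through BP_Enemy's TargetPoint array and wraps around, but it never runs.
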(event EventReceiveExecuteAI
  (params (OwnerController :type AI%20Controller%20Object%20Reference) (ControlledPawn :type Pawn%20Object%20Reference))
  (AI|BehaviorTree|SetBlackboardValueasVector (Variables|Default|GetBBloc) (.RandomLocation (AI|Navigation|GetRandomReachablePointinRadius (Transformation|GetActorLocation OwnerController) 2e+03 0 0)))
  (AI|BehaviorTree|FinishExecute true))